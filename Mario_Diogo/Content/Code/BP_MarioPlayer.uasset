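; BP_MarioPlayer is a Mario-style side-scrolling player whose mesh and capsule are constrained to the YZ plane.
; Input axes offset its location along Y, while Jump01 applies an upward capsule impulse when a downward sphere trace hits.
; Death shows the losing widget, calls Jump01 twice and destroys the actor after a delay, which reloads the level.
; It also prints Score every tick, and PowerUp/PowerDown switch the capsule between half and full scale.
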(event Custom|Death
  (Utilities|FlowControl|Sequence
    (:then_0
      (bind _returnvalue (UserInterface|CreateWidget "/Game/Widgets/WD_Losing.WD_Losing_C"))
      (UserInterface|Viewport|AddtoViewport _returnvalue 0)
      (Utilities|FlowControl|Delay 1.3)
      (Actor|DestroyActor))
    (:then_1
      (CallFunction|Jump01)
      (CallFunction|Jump01))))

(event EventTick
  (params (DeltaSeconds :type Float%20%28single-precision%29))
  (Development|PrintString (Utilities|String|Append "Score:" (Utilities|String|ToString(Integer) (Variables|Default|GetScore))) true true "(R=0.000000,G=0.660000,B=1.000000,A=1.000000)" 0.0))

(event EventBeginPlay
  (Class|PrimitiveComponent|SetConstraintMode (Variables|Character|GetMesh) "YZPlane"))

(event EventDestroyed
  (bind _returnvalue (Game|GetCurrentLevelName true))
  (Game|OpenLevel(byName) (Utilities|String|StringToName _returnvalue)))

(event Input|ActionEvents|InputActionJump
  (params (Key :type Key%20Structure :default "None"))
  (:Pressed
    (CallFunction|Jump01)))

(event Input|AxisEvents|InputAxisMOveRight
  (params (AxisValue :type Float%20%28single-precision%29))
  (Transformation|SetActorLocation (+ (* (* (Math|Vector|MakeVector 0.0 (Variables|Components|GetWalkSpeed) 0.0) AxisValue) (Utilities|Time|GetWorldDeltaSeconds)) (Transformation|GetActorLocation)) false false))

(event Input|AxisEvents|InputAxisMoveLeft
  (params (AxisValue :type Float%20%28single-precision%29))
  (Transformation|SetActorLocation (+ (* (* (Math|Vector|MakeVector 0.0 (Variables|Components|GetWalkSpeed) 0.0) AxisValue) (Utilities|Time|GetWorldDeltaSeconds)) (Transformation|GetActorLocation)) false false))

(fn ConstructionScript)

(fn NewFunction0)

(fn Jump01
  (bind _returnvalue (Transformation|GetActorLocation))
  (bind _capsulecomponent (Variables|Collision|GetCapsuleComponent))
  (Development|PrintString "Jump Pressed")
  (bind _returnvalue_2 (Collision|SphereTraceByChannel _returnvalue (- _returnvalue (Math|Vector|MakeVector 0.0 0.0 (Variables|/Script/Engine.CapsuleComponent|GetCapsuleHalfHeight _capsulecomponent))) (Variables|/Script/Engine.CapsuleComponent|GetCapsuleRadius _capsulecomponent) "TraceTypeQuery1" false 0 "ForDuration" true "(R=1.000000,G=0.000000,B=0.000000,A=1.000000)" "(R=0.000000,G=1.000000,B=0.000000,A=1.000000)" 1.0))
  (if _returnvalue_2
    (Physics|AddImpulse (Variables|Collision|GetCapsuleComponent) (Math|Vector|MakeVector 0.0 0.0 (Variables|Components|GetJumpForce)) "None" true)
    (Development|PrintString "Mario Jump!")))

(fn PowerUp
  (Transformation|SetWorldScale3D (Variables|Collision|GetCapsuleComponent) "0.500000,0.500000,0.500000"))

(fn PowerDown
  (Transformation|SetWorldScale3D (Variables|Collision|GetCapsuleComponent) "1.000000,1.000000,1.000000"))