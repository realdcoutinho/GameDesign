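; BP_DoorSwitch is a sliding door that stays locked, when IsLocked is set, until its linked switch is pressed.
; The switch event clears IsLocked and turns the lock light from red to green; the construction script also sets that color from the lock state.
; A box overlap enables input for BP_Mario, so E plays the DoorAnimation timeline to slide the unlocked door.
; Leaving the box disables input and reverses the timeline.
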(event OnComponentBeginOverlap(box)
  (params (OverlappedComponent :type Primitive%20Component%20Object%20Reference) (OtherActor :type Actor%20Object%20Reference) (OtherComp :type Primitive%20Component%20Object%20Reference) (OtherBodyIndex :type Integer) (bFromSweep :type Boolean) (SweepResult :type Hit%20Result%20Structure%20%28by%20ref%29))
  (Utilities|Casting|CastToBP_Mario OtherActor)
  (Input|EnableInput (Game|GetPlayerController 0)))

(event OnComponentEndOverlap(box)
  (params (OverlappedComponent :type Primitive%20Component%20Object%20Reference) (OtherActor :type Actor%20Object%20Reference) (OtherComp :type Primitive%20Component%20Object%20Reference) (OtherBodyIndex :type Integer))
  (Utilities|Casting|CastToBP_Mario OtherActor)
  (Input|DisableInput (Game|GetPlayerController 0))
  (bind _door_sliding (Timeline|Door%20animation Reverse)
    (:Update
      (Transformation|SetRelativeLocation (Variables|Default|Getdoor) _door_sliding false false))))

(event Custom|UnlockDoor
  (params (switch :type BP%20Switch%20Object%20Reference))
  (bind _locklight (Variables|Default|GetLockLight))
  (if (== switch (Variables|Default|GetSwitch))
    (bind _output_get (Variables|Default|SetIsLocked false))
    (if _output_get
      (Rendering|Components|Light|SetLightColor _locklight "(R=1.000000,G=0.000000,B=0.000000,A=1.000000)" true)
      (else
        (Rendering|Components|Light|SetLightColor _locklight "(R=0.032487,G=1.000000,B=0.000000,A=1.000000)" true)))))

(event EventBeginPlay
  (EventDispatchers|BindEventtoSwitchPressed (Variables|Default|GetSwitch) (delegate Custom|UnlockDoor)))

(event Input|KeyboardEvents|E
  (params (Key :type Key%20Structure :default "None"))
  (:Pressed
    (if (not (Variables|Default|GetIsLocked))
      (bind _door_sliding (Timeline|Door%20animation Play)
        (:Update
          (Transformation|SetRelativeLocation (Variables|Default|Getdoor) _door_sliding false false))))))

(fn ConstructionScript
  (bind _locklight (Variables|Default|GetLockLight))
  (if (Variables|Default|GetIsLocked)
    (Rendering|Components|Light|SetLightColor _locklight "(R=1.000000,G=0.000000,B=0.000000,A=1.000000)" true)
    (else
      (Rendering|Components|Light|SetLightColor _locklight "(R=0.032487,G=1.000000,B=0.000000,A=1.000000)" true))))