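; BP_Enemy is a Mario-style patrolling enemy that kills the player on contact and dies when stomped.
; Tick moves it along a stored direction, which the Hit event flips between -Y and +Y.
; WeaponSpot overlap calls Mario's Death, while WeakSpot overlap calls his Jump0, squashes the capsule and destroys the enemy.
; IsHit and IsKilled flags keep the two outcomes mutually exclusive, and IsHit also halts movement.
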(event OnComponentBeginOverlap(WeakSpot)
  (params (OverlappedComponent :type Primitive%20Component%20Object%20Reference) (OtherActor :type Actor%20Object%20Reference) (OtherComp :type Primitive%20Component%20Object%20Reference) (OtherBodyIndex :type Integer) (bFromSweep :type Boolean) (SweepResult :type Hit%20Result%20Structure%20%28by%20ref%29))
  (bind _asbp_mario (Utilities|Casting|CastToBP_Mario OtherActor))
  (if (not (Variables|Default|GetIsKilled))
    (Utilities|FlowControl|Sequence
      (:then_0
        (Utilities|FlowControl|DoOnce false
          (:Completed
            (Default|Jump0 _asbp_mario)
            (Transformation|SetWorldScale3D (Variables|Collision|GetCapsuleComponent) "1.000000,1.000000,0.300000")
            (Utilities|FlowControl|Delay 0.3)
            (Actor|DestroyActor))))
      (:then_1
        (Variables|Default|SetIsHit true)))))

(event OnComponentBeginOverlap(WeaponSpot)
  (params (OverlappedComponent :type Primitive%20Component%20Object%20Reference) (OtherActor :type Actor%20Object%20Reference) (OtherComp :type Primitive%20Component%20Object%20Reference) (OtherBodyIndex :type Integer) (bFromSweep :type Boolean) (SweepResult :type Hit%20Result%20Structure%20%28by%20ref%29))
  (Utilities|FlowControl|Sequence
    (:then_0
      (bind _asbp_mario (Utilities|Casting|CastToBP_Mario OtherActor))
      (if (not (Variables|Default|GetIsHit))
        (Utilities|FlowControl|DoOnce false :!label _label
          (:Completed
            (Variables|Default|SetIsKilled true)
            (Default|Death _asbp_mario)
            (Utilities|FlowControl|Delay 1.0)
            (goto _label Reset)))))))

(event EventTick
  (params (DeltaSeconds :type Float%20%28single-precision%29))
  (if (not (Variables|Default|GetIsHit))
    (Pawn|Input|AddMovementInput (Variables|Default|GetDelta%20Seconds) 0.4 false)))

(event Collision|EventHit
  (params (MyComp :type Primitive%20Component%20Object%20Reference) (Other :type Actor%20Object%20Reference) (OtherComp :type Primitive%20Component%20Object%20Reference) (bSelfMoved :type Boolean) (HitLocation :type Vector :default "0, 0, 0") (HitNormal :type Vector :default "0, 0, 0") (NormalImpulse :type Vector :default "0, 0, 0") (Hit :type Hit%20Result%20Structure%20%28by%20ref%29))
  (if (not (Variables|Default|GetIsHit))
    (Utilities|FlowControl|FlipFlop
      (:A
        (Variables|Default|SetDelta%20Seconds "0,-1.000000, 0"))
      (:B
        (Variables|Default|SetDelta%20Seconds "0,1.000000, 0")))))

(event EventBeginPlay
  (Variables|Default|SetIsHit false)
  (Variables|Default|SetIsKilled false))

(fn ConstructionScript)