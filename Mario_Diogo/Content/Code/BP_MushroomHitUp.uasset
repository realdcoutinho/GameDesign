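; BP_MushroomHitUp is a one-time hit block that releases a BP_MushroomUp when BP_Mario or BP_MarioPlayer overlaps its box.
; Both casts feed a shared DoOnce that eases the root component upward with MoveComponentTo.
; After the rise, it spawns the mushroom at the arrow's transform with a default controller, while the root drops back down after a short delay.
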(event OnComponentBeginOverlap(Box)
  (params (OverlappedComponent :type Primitive%20Component%20Object%20Reference) (OtherActor :type Actor%20Object%20Reference) (OtherComp :type Primitive%20Component%20Object%20Reference) (OtherBodyIndex :type Integer) (bFromSweep :type Boolean) (SweepResult :type Hit%20Result%20Structure%20%28by%20ref%29))
  (bind _defaultsceneroot (Variables|Default|GetDefaultSceneRoot))
  (bind _defaultsceneroot_2 (Variables|Default|GetDefaultSceneRoot))
  (bind _returnvalue (Transformation|GetRelativeTransform _defaultsceneroot))
  (Utilities|FlowControl|Sequence
    (:then_0
      (Utilities|Casting|CastToBP_Mario OtherActor))
    (:then_1
      (Utilities|Casting|CastToBP_MarioPlayer OtherActor)))
  (Utilities|FlowControl|DoOnce false
    (:Completed
      (Components|MoveComponentTo _defaultsceneroot_2 (+ (.location (Transformation|GetRelativeTransform _defaultsceneroot_2)) "0, 0,30.000000") (Math|Rotator|MakeRotator 0.0 0.0 0.0) true true 0.3 false)
      (Utilities|FlowControl|Sequence
        (:then_0
          (Utilities|FlowControl|Delay 0.11)
          (Components|MoveComponentTo _defaultsceneroot (+ (.location _returnvalue) "0, 0,-30.000000") (.rotation _returnvalue) false false 0.3 false))
        (:then_1
          (bind _returnvalue_2 (Game|SpawnActorfromClass "/Game/Code/BP_MushroomUp.BP_MushroomUp_C" (Transformation|GetWorldTransform (Variables|Default|GetArrow)) "Undefined" 0 0))
          (Pawn|SpawnDefaultController _returnvalue_2))))))

(event EventBeginPlay)

(event Collision|EventActorBeginOverlap
  (params (OtherActor :type Actor%20Object%20Reference)))

(event EventTick
  (params (DeltaSeconds :type Float%20%28single-precision%29)))

(fn ConstructionScript)