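; BP_Mario is a Mario player character that moves sideways and jumps from player input.
; Left and right axis inputs offset the actor along world Y by WalkSpeed and delta time, setting location directly without sweep.
; Jump uses a downward sphere trace sized from the capsule as a ground check, then applies an upward velocity-change impulse to the capsule.
; Debug prints and trace drawing remain in the jump logic.
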(event EventBeginPlay)

(event Collision|EventActorBeginOverlap
  (params (OtherActor :type Actor%20Object%20Reference)))

(event EventTick
  (params (DeltaSeconds :type Float%20%28single-precision%29)))

(event Input|ActionEvents|InputActionJump
  (params (Key :type Key%20Structure :default "None"))
  (:Pressed
    (CallFunction|Jump)))

(event Input|AxisEvents|InputAxisMOveRight
  (params (AxisValue :type Float%20%28single-precision%29))
  (Transformation|SetActorLocation (+ (* (* (Math|Vector|MakeVector 0.0 (Variables|Default|GetWalkSpeed) 0.0) AxisValue) (Utilities|Time|GetWorldDeltaSeconds)) (Transformation|GetActorLocation)) false false))

(event Input|AxisEvents|InputAxisMoveLeft
  (params (AxisValue :type Float%20%28single-precision%29))
  (Transformation|SetActorLocation (+ (* (* (Math|Vector|MakeVector 0.0 (Variables|Default|GetWalkSpeed) 0.0) AxisValue) (Utilities|Time|GetWorldDeltaSeconds)) (Transformation|GetActorLocation)) false false))

(fn ConstructionScript)

(fn Jump
  (bind _returnvalue (Transformation|GetActorLocation))
  (bind _capsule (Variables|Default|GetCapsule))
  (Development|PrintString "Jump Pressed")
  (bind _returnvalue_2 (Collision|SphereTraceByChannel _returnvalue (- _returnvalue (Math|Vector|MakeVector 0.0 0.0 (Variables|/Script/Engine.CapsuleComponent|GetCapsuleHalfHeight _capsule))) (Variables|/Script/Engine.CapsuleComponent|GetCapsuleRadius _capsule) "TraceTypeQuery1" false 0 "ForDuration" true "(R=1.000000,G=0.000000,B=0.000000,A=1.000000)" "(R=0.000000,G=1.000000,B=0.000000,A=1.000000)" 1.0))
  (if _returnvalue_2
    (Physics|AddImpulse (Variables|Default|GetCapsule) (Math|Vector|MakeVector 0.0 0.0 (Variables|Default|GetJumpForce)) "None" true)
    (Development|PrintString "Mario Jump!")))