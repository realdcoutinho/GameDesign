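; BP_Goomba is a Mario-style patrolling enemy that can be stomped.
; Tick moves it along MoveDirection, reversing when it passes either TargetLeft or TargetRight on Y, both detached at BeginPlay.
; WeakSpot overlap makes Mario jump, sets IsHit to stop movement, squashes the Box and destroys the Goomba after a short delay.
; Weapon overlap destroys Mario only if IsHit is set, otherwise setting IsKilled; coin spawning is unwired.
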(event OnComponentBeginOverlap(Weapon)
  (params (OverlappedComponent :type Primitive%20Component%20Object%20Reference) (OtherActor :type Actor%20Object%20Reference) (OtherComp :type Primitive%20Component%20Object%20Reference) (OtherBodyIndex :type Integer) (bFromSweep :type Boolean) (SweepResult :type Hit%20Result%20Structure%20%28by%20ref%29))
  (Utilities|FlowControl|Sequence
    (:then_0
      (bind _asbp_mario (Utilities|Casting|CastToBP_Mario OtherActor))
      (if (Variables|Default|GetIsHit?)
        (Actor|DestroyActor _asbp_mario)
        (else
          (Variables|Default|SetIsKilled true))))))

(event OnComponentBeginOverlap(WeakSpot)
  (params (OverlappedComponent :type Primitive%20Component%20Object%20Reference) (OtherActor :type Actor%20Object%20Reference) (OtherComp :type Primitive%20Component%20Object%20Reference) (OtherBodyIndex :type Integer) (bFromSweep :type Boolean) (SweepResult :type Hit%20Result%20Structure%20%28by%20ref%29))
  (bind _asbp_mario (Utilities|Casting|CastToBP_Mario OtherActor))
  (Default|Jump0 _asbp_mario)
  (Utilities|FlowControl|Sequence
    (:then_0
      (Transformation|SetWorldScale3D (Variables|Default|GetBox) "1.000000,1.000000,0.500000")
      (Utilities|FlowControl|Sequence
        (:then_0
          (Utilities|FlowControl|Delay 0.2)
          (Components|DestroyComponent (Variables|Default|GetBox))
          (Actor|DestroyActor))))
    (:then_1
      (Variables|Default|SetIsHit? true))))

(event EventBeginPlay
  (Variables|Default|SetIsHit? false)
  (Transformation|DetachFromComponent (Variables|Default|GetTarget_Left) "KeepWorld" "KeepWorld" "KeepWorld" true)
  (Transformation|DetachFromComponent (Variables|Default|GetTarget_Right) "KeepWorld" "KeepWorld" "KeepWorld" true))

(event EventTick
  (params (DeltaSeconds :type Float%20%28single-precision%29))
  ;[1 1 1] If hit, stop movement
  (if (not (Variables|Default|GetIsHit?))
    (Transformation|SetActorLocation (+ (* (Variables|Default|GetMoveDirection) (* DeltaSeconds (Variables|Default|GetMoveSpeed))) (Transformation|GetActorLocation)) false false)
    (Utilities|FlowControl|Sequence
      (:then_0
        (if (and (CallFunction|IsMovingRight) (CallFunction|IsPastRightTarget))
          (CallFunction|InvertMovement)))
      (:then_1
        (if (and (CallFunction|IsMovingLeft) (CallFunction|IsPastLeftTarget))
          (CallFunction|InvertMovement))))))

(fn ConstructionScript)

(fn InvertMovement
  (Variables|Default|SetMoveDirection (* (Variables|Default|GetMoveDirection) -1.0)))

(fn IsMovingRight
  (return (> (.y (Variables|Default|GetMoveDirection)) 0.0)))

(fn IsPastRightTarget
  (return (> (.y (Transformation|GetActorLocation)) (.y (Transformation|GetWorldLocation (Variables|Default|GetTarget_Right))))))

(fn IsMovingLeft
  (return (< (.y (Variables|Default|GetMoveDirection)) 0.0)))

(fn IsPastLeftTarget
  (return (< (.y (Transformation|GetActorLocation)) (.y (Transformation|GetWorldLocation (Variables|Default|GetTarget_Left))))))