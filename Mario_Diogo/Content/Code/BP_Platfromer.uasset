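; BP_Platfromer respawns the player's BP_Mario character whenever it is destroyed.
; On BeginPlay it casts the player character to BP_Mario and binds to its OnDestroyed event.
; After a short delay, the handler spawns a new BP_Mario at SpawnTransform and has the player controller possess it.
; It then calls Respawn to bind to the new character, so the cycle repeats on each death.
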(event Custom|Destroyed
  (params (DestroyedActor :type Actor%20Object%20Reference))
  (Utilities|FlowControl|Delay 2.0)
  (bind _returnvalue (Game|SpawnActorfromClass "/Game/Code/BP_Mario.BP_Mario_C" (Variables|Default|GetSpawn%20Transform) "Undefined" 0 0))
  (Pawn|Possess (Game|GetPlayerController 0) _returnvalue)
  (CallFunction|Respawn))

(event Custom|Respawn
  (bind _asbp_mario (Utilities|Casting|CastToBP_Mario (Game|GetPlayerCharacter 0)))
  (Game|BindEventtoOnDestroyed _asbp_mario (delegate Custom|Destroyed)))

(event EventBeginPlay
  (bind _asbp_mario (Utilities|Casting|CastToBP_Mario (Game|GetPlayerCharacter 0)))
  (Game|BindEventtoOnDestroyed _asbp_mario (delegate Custom|Destroyed)))

(event EventTick
  (params (DeltaSeconds :type Float%20%28single-precision%29)))

(fn ConstructionScript)