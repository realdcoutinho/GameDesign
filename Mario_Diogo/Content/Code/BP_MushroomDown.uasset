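; BP_MushroomDown is a moving mushroom pickup that powers down Mario on contact.
; Tick constantly feeds movement input along a stored direction vector, misleadingly named DeltaSeconds, and each Hit event flip-flops that vector between negative and positive Y.
; Overlapping its collision component casts to either BP_Mario or BP_MarioPlayer, calls PowerDown on the match, then destroys the mushroom.
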(event OnComponentBeginOverlap(collison)
  (params (OverlappedComponent :type Primitive%20Component%20Object%20Reference) (OtherActor :type Actor%20Object%20Reference) (OtherComp :type Primitive%20Component%20Object%20Reference) (OtherBodyIndex :type Integer) (bFromSweep :type Boolean) (SweepResult :type Hit%20Result%20Structure%20%28by%20ref%29))
  (Utilities|FlowControl|Sequence
    (:then_0
      (bind _asbp_mario (Utilities|Casting|CastToBP_Mario OtherActor))
      (Default|PowerDown _asbp_mario))
    (:then_1
      (bind _asbp_mario_player (Utilities|Casting|CastToBP_MarioPlayer OtherActor))
      (Default|PowerDown _asbp_mario_player)))
  (Actor|DestroyActor))

(event EventTick
  (params (DeltaSeconds :type Float%20%28single-precision%29))
  (Pawn|Input|AddMovementInput (Variables|Default|GetDelta%20Seconds) 0.4 false))

(event Collision|EventHit
  (params (MyComp :type Primitive%20Component%20Object%20Reference) (Other :type Actor%20Object%20Reference) (OtherComp :type Primitive%20Component%20Object%20Reference) (bSelfMoved :type Boolean) (HitLocation :type Vector :default "0, 0, 0") (HitNormal :type Vector :default "0, 0, 0") (NormalImpulse :type Vector :default "0, 0, 0") (Hit :type Hit%20Result%20Structure%20%28by%20ref%29))
  (Utilities|FlowControl|FlipFlop
    (:A
      (Variables|Default|SetDelta%20Seconds "0,-1.000000, 0"))
    (:B
      (Variables|Default|SetDelta%20Seconds "0,1.000000, 0"))))

(fn ConstructionScript)