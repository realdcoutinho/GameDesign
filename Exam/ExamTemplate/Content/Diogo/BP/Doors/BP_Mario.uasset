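; Mario-style player pawn that moves along the Y axis, prints its Score every tick and reloads the current level when destroyed.
; MoveRight offsets location without sweep; MoveLeft is empty.
; Jump0 applies an upward capsule impulse after a downward sphere-trace ground check, and is called only by Death, twice; Death's widget and destroy chain is disconnected.
; PowerUp halves the capsule's Z scale and PowerDown restores it.
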(event Custom|Death
  (Utilities|FlowControl|Sequence
    (:then_1
      (CallFunction|Jump0)
      (CallFunction|Jump0))))

(event Collision|EventActorBeginOverlap
  (params (OtherActor :type Actor%20Object%20Reference)))

(event EventTick
  (params (DeltaSeconds :type Float%20%28single-precision%29))
  (Development|PrintString (Utilities|String|Append "Score:" (Utilities|String|ToString(Integer) (Variables|Default|GetScore))) true true "(R=0.000000,G=0.660000,B=1.000000,A=1.000000)" 0.0))

(event EventDestroyed
  (bind _returnvalue (Game|GetCurrentLevelName true))
  (Game|OpenLevel(byName) (Utilities|String|StringToName _returnvalue)))

(event Input|ActionEvents|InputActionJump
  (params (Key :type Key%20Structure :default "None")))

(event Input|AxisEvents|InputAxisMOveRight
  (params (AxisValue :type Float%20%28single-precision%29))
  (Transformation|SetActorLocation (+ (* (* (Math|Vector|MakeVector 0.0 (Variables|Default|GetWalkSpeed) 0.0) AxisValue) (Utilities|Time|GetWorldDeltaSeconds)) (Transformation|GetActorLocation)) false false))

(event Input|AxisEvents|InputAxisMoveLeft
  (params (AxisValue :type Float%20%28single-precision%29)))

(fn ConstructionScript)

(fn Jump0
  (bind _returnvalue (Transformation|GetActorLocation))
  (bind _capsule (Variables|Default|GetCapsule))
  (Development|PrintString "Jump Pressed")
  (bind _returnvalue_2 (Collision|SphereTraceByChannel _returnvalue (- _returnvalue (Math|Vector|MakeVector 0.0 0.0 (Variables|/Script/Engine.CapsuleComponent|GetCapsuleHalfHeight _capsule))) (Variables|/Script/Engine.CapsuleComponent|GetCapsuleRadius _capsule) "TraceTypeQuery1" false 0 "ForDuration" true "(R=1.000000,G=0.000000,B=0.000000,A=1.000000)" "(R=0.000000,G=1.000000,B=0.000000,A=1.000000)" 1.0))
  (if _returnvalue_2
    (Physics|AddImpulse (Variables|Default|GetCapsule) (Math|Vector|MakeVector 0.0 0.0 (Variables|Default|GetJumpForce)) "None" true)
    (Development|PrintString "Mario Jump!")))

(fn PowerUp
  (Transformation|SetWorldScale3D (Variables|Default|GetCapsule) "1.000000,1.000000,0.500000"))

(fn PowerDown
  (Transformation|SetWorldScale3D (Variables|Default|GetCapsule) "1.000000,1.000000,1.000000"))