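; BP_DoorKeyCard is a sliding door that a player holding the matching key card can open.
; When BP_Player enters the Box trigger, it enables input if the player's KeyCard array is true at index KeyCardValue.
; Pressing E plays the DoorAnimation timeline, which moves the Door's relative location.
; Leaving the box disables input and reverses the timeline to close the door.
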(event OnComponentBeginOverlap(box)
  (params (OverlappedComponent :type Primitive%20Component%20Object%20Reference) (OtherActor :type Actor%20Object%20Reference) (OtherComp :type Primitive%20Component%20Object%20Reference) (OtherBodyIndex :type Integer) (bFromSweep :type Boolean) (SweepResult :type Hit%20Result%20Structure%20%28by%20ref%29))
  (bind _asbp_player (Utilities|Casting|CastToBP_Player OtherActor))
  (for (_array_element _array_index) (Variables|/Game/Diogo/BP/BP_Player.BP_Player_C|GetKeyCard _asbp_player)
    (if (and _array_element (== _array_index (Variables|Default|GetKeyCard_Value)))
      (Input|EnableInput (Game|GetPlayerController 0)))))

(event OnComponentEndOverlap(box)
  (params (OverlappedComponent :type Primitive%20Component%20Object%20Reference) (OtherActor :type Actor%20Object%20Reference) (OtherComp :type Primitive%20Component%20Object%20Reference) (OtherBodyIndex :type Integer))
  (Utilities|Casting|CastToBP_Player OtherActor)
  (Input|DisableInput (Game|GetPlayerController 0))
  (bind _door_sliding (Timeline|Door%20animation Reverse)
    (:Update
      (Transformation|SetRelativeLocation (Variables|Default|Getdoor) _door_sliding false false))))

(event Input|KeyboardEvents|E
  (params (Key :type Key%20Structure :default "None"))
  (:Pressed
    (Development|PrintString "Hello")
    (bind _door_sliding (Timeline|Door%20animation Play)
      (:Update
        (Transformation|SetRelativeLocation (Variables|Default|Getdoor) _door_sliding false false)))))

(fn ConstructionScript)