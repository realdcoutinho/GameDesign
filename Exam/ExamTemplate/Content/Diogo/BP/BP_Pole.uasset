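; BP_Pole is a keycard-gated barrier that slides its static mesh once the player holds the matching keycard.
; Every Tick it fetches BP_Player and loops through its KeyCard boolean array for a true entry at the index equal to KayCardValue.
; A match plays a timeline whose DoorSliding track sets the mesh's relative location, with no proximity check or reverse.
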(event EventBeginPlay)

(event Collision|EventActorBeginOverlap
  (params (OtherActor :type Actor%20Object%20Reference)))

(event EventTick
  (params (DeltaSeconds :type Float%20%28single-precision%29))
  (bind _returnvalue (Actor|GetActorOfClass "/Game/Diogo/BP/BP_Player.BP_Player_C"))
  (for (_array_element _array_index) (Variables|/Game/Diogo/BP/BP_Player.BP_Player_C|GetKeyCard _returnvalue)
    (Utilities|FlowControl|Sequence
      (:then_0
        (if (and _array_element (== _array_index (Variables|Default|GetKayCard_Value)))
          (bind _door_sliding (Timeline|Timeline_0 Play)
            (:Update
              (Transformation|SetRelativeLocation (Variables|Debug|GetStaticMeshComponent) _door_sliding false false))))))))

(fn ConstructionScript)