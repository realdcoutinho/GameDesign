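; BP_EnergyBox is a rechargeable energy station that gives the player a battery when touched.
; Overlapping the collision while charged increments BP_Player's NumBateries, plays a synth sound, clears Charge and switches the three antennas from blue to red.
; While discharged, Tick runs a 20-second Delay that then restores the charge and blue antennas.
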(event OnComponentBeginOverlap(Collison)
  (params (OverlappedComponent :type Primitive%20Component%20Object%20Reference) (OtherActor :type Actor%20Object%20Reference) (OtherComp :type Primitive%20Component%20Object%20Reference) (OtherBodyIndex :type Integer) (bFromSweep :type Boolean) (SweepResult :type Hit%20Result%20Structure%20%28by%20ref%29))
  (if (Variables|Default|GetCharge?)
    (bind _asbp_player (Utilities|Casting|CastToBP_Player OtherActor))
    (Utilities|FlowControl|Sequence
      (:then_0
        (Rendering|SetVisibility (Variables|Default|GetAntena2%20blue) false false))
      (:then_1
        (Variables|Default|SetCharge? false))
      (:then_2
        (Rendering|SetVisibility (Variables|Default|GetAntena2%20red) true false))
      (:then_3
        (bind _result (Math|Integer|IncrementInt (Variables|/Game/Diogo/BP/BP_Player.BP_Player_C|GetNumBateries _asbp_player))
          (:%20%20
            (Variables|/Game/Diogo/BP/BP_Player.BP_Player_C|SetNumBateries _asbp_player _result))))
      (:then_4
        (Audio|PlaySound2D "/Game/Data/SoundEffects/S_Synth01.S_Synth01" 1.0 1.0 0.0 0 0)))))

(event EventTick
  (params (DeltaSeconds :type Float%20%28single-precision%29))
  (if (not (Variables|Default|GetCharge?))
    (Utilities|FlowControl|Delay 2e+01)
    (Utilities|FlowControl|Sequence
      (:then_0
        (Rendering|SetVisibility (Variables|Default|GetAntena2%20blue) true false))
      (:then_1
        (Variables|Default|SetCharge? true))
      (:then_2
        (Rendering|SetVisibility (Variables|Default|GetAntena2%20red) false false)))))

(fn ConstructionScript)